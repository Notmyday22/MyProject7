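; Coin is a collectible pickup actor that spins in the level and adds to the player's coin count.
; Tick rolls the static mesh by a fixed step each frame, without delta-time scaling.
; Any actor overlap plays a 2D explosion sound, increments CoinCounter on player 0's ThirdPersonCharacter regardless of which actor overlapped, then destroys the coin.
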(event EventBeginPlay)

(event Collision|EventActorBeginOverlap
  (params (OtherActor :type Actor%20Object%20Reference))
  ;[1 1 1] Coin Pickup
  (Audio|PlaySound2D "/Game/StarterContent/Audio/Explosion01.Explosion01" 1.0 1.0 0.0 0 0)
  (bind _asthird_person_character (Utilities|Casting|CastToThirdPersonCharacter (Game|GetPlayerCharacter 0)))
  (Variables|/Game/ThirdPersonBP/Blueprints/ThirdPersonCharacter.ThirdPersonCharacter_C|SetCoinCounter _asthird_person_character (+ (Variables|/Game/ThirdPersonBP/Blueprints/ThirdPersonCharacter.ThirdPersonCharacter_C|GetCoinCounter _asthird_person_character) 1))
  (Actor|DestroyActor))

(event EventTick
  (params (DeltaSeconds :type Float%20%28single-precision%29))
  (bind _staticmesh (Variables|Default|GetStaticMesh))
  (bind _relativerotation (Variables|/Script/Engine.SceneComponent|GetRelativeRotation _staticmesh))
  ;[1 1 1] Coin Spinning
  (Transformation|SetRelativeRotation _staticmesh (Math|Rotator|MakeRotator (+ (.roll _relativerotation) 2.5) (.pitch _relativerotation) (.yaw _relativerotation)) false false))

(fn ConstructionScript)